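; Effect manager Blueprint that spawns Niagara effects by effect type and returns the spawned system.
; FindEffect searches the EffectsConfigs array for the entry matching the requested type and returns its effect asset.
; SpawnEffect passes that asset to an attached spawn with relative offset when a validity check succeeds, otherwise to a spawn at location.
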(fn `FindEffect`
  (params (EffectType :type "/Game/Blueprints/Enum/EffectType Enum" :default "NewEnumerator0"))
  (returns (EffectConfig :type "NiagaraSystem Object Reference"))
  (for _array_element (`self.EffectsConfigs`)
    (bind (_effecttype _effect) (break `/Game/Blueprints/Structure/EffectConfig` _array_element))
    (if (`|EnumEquality` _effecttype EffectType)
      (return _effect))))

(fn `SpawnEffect`
  (params (EffectType :type "/Game/Blueprints/Enum/EffectType Enum" :default "NewEnumerator0"))
  (returns (Effect :type "NiagaraComponent Object Reference"))
  (locals (_SpawnEffectConfig :type " Structure") (FindEffectConfig :type " Structure") (EffectReturn :type "NiagaraComponent Object Reference"))
  (bind _effectconfig (`self.FindEffect` EffectType))
  (`/Engine/EditorBlueprintResources/StandardMacros.IsValid` null
    (:`Is Valid`
      (bind _returnvalue (`NiagaraFunctionLibrary.SpawnSystemAttached` _effectconfig null "None" (0.0 0.0 0.0) (struct) "KeepRelativeOffset"))
      (set `local.EffectReturn` _returnvalue))
    (:`Is Not Valid`
      (bind _returnvalue_2 (`NiagaraFunctionLibrary.SpawnSystemAtLocation` _effectconfig))
      (set `local.EffectReturn` _returnvalue_2)))
  (return (`local.EffectReturn`)))

(fn `UserConstructionScript`
  (locals (Effects :type Boolean)))